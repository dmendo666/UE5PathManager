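; Humanoid character Blueprint that relays path start and end events to its animation Blueprint.
; BeginPlay casts the mesh's anim instance to humanoid_AnimationBP and caches it.
; The start and end path events both call ToggleAnimation, which writes the Walking flag and Alpha value to that instance.
; Both events pass Walking as false, so only the supplied Alpha differs between calls.
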(event Custom|startCharacterPath_Event
  (params (alpha :type Enum_KeyInput%20Enum :default "NewEnumerator0"))
  (CallFunction|ToggleAnimation false alpha))

(event Custom|endCharacterPath_Event
  (params (alpha :type Enum_KeyInput%20Enum :default "NewEnumerator0"))
  (CallFunction|ToggleAnimation false alpha))

(event EventBeginPlay
  (bind _ashumanoid_animation_bp (Utilities|Casting|CastTohumanoid_AnimationBP (Components|SkeletalMesh|GetAnimInstance (Variables|Character|GetMesh))))
  (Variables|Default|SetanimationBP _ashumanoid_animation_bp))

(event Collision|EventActorBeginOverlap
  (params (OtherActor :type Actor%20Object%20Reference)))

(event EventTick
  (params (DeltaSeconds :type Float%20%28single-precision%29)))

(fn ConstructionScript)

(fn ToggleAnimation
  (params (toWalk :type Boolean) (alpha :type Enum_KeyInput%20Enum :default "NewEnumerator0"))
  (bind _animationbp (Variables|Default|GetanimationBP))
  (Variables|/Game/GeneralResources/humanoid/humanoid_AnimationBP.humanoid_AnimationBP_C|Setwalking _animationbp toWalk)
  (Variables|/Game/GeneralResources/humanoid/humanoid_AnimationBP.humanoid_AnimationBP_C|Setalpha _animationbp alpha))